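; Enemy AI controller that sends its controlled pawn toward one random nearby point when play begins.
; GetRandomTarget logs the pawn's name and returns its location offset randomly in X and Y within plus or minus Range, keeping the same height.
; BeginPlay stores that point as TargetPosition, issues a single MoveToLocation with pathfinding disabled, then prints the position.
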(event `self.ReceiveBeginPlay`
  (bind _returnvalue (`self.GetRandomTarget`))
  (bind _output_get (set `self.TargetPosition` _returnvalue))
  (`self.MoveToLocation` _output_get -1.0 true false false true null)
  (`KismetSystemLibrary.PrintString` (`KismetStringLibrary.Conv_VectorToString` _output_get)))

(fn `GetRandomTarget`
  (returns (ReturnValue :type "Vector Structure"))
  (bind _returnvalue (`self.K2_GetPawn`))
  (bind _range (`self.Range`))
  (bind _range_2 (`self.Range`))
  (`|ExecutionSequence`
    (:`then_0`
      (`KismetSystemLibrary.PrintString` (`KismetStringLibrary.Concat_StrStr` "I am the controlled pawn:" (`KismetSystemLibrary.GetDisplayName` _returnvalue))))
    (:`then_1`
      (return (+ (`self.K2_GetActorLocation` _returnvalue) (`KismetMathLibrary.MakeVector` (`KismetMathLibrary.RandomFloatInRange` (* _range_2 -1.0) _range_2) (`KismetMathLibrary.RandomFloatInRange` (* _range -1.0) _range)))))))

(fn `UserConstructionScript`)